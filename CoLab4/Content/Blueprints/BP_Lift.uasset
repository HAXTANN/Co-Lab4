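; Lift actor that moves its body vertically between two levels along a timeline when a player interacts at its switch.
; Overlapping the switch trigger with a Character enables input and shows an interact widget, both undone on exit.
; MoveLift plays or reverses the timeline based on OnTopFloor, which is only ever set true.
; Meshes tagged LiftSwitch glow during travel and turn red when it finishes.
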(event `MoveLift`
  ;[0.08228 0.09759 0.15 0.502] LiftLoop
  ;;[0.08228 0.09759 0.15 0.502] Turn Lights Blue
  (if (`self.OnTopFloor?`)
    (for _ (`self.MeshesToUpdate`)
      (`PrimitiveComponent.SetMaterial` (`self.MeshesToUpdate`) 0 "/Game/Materials/M_GlowingMaterial.M_GlowingMaterial")
      ;;[0.08228 0.09759 0.15 0.502] Play = Move up Reversed = Move Down
      (bind (_direction _alpha) (`Timeline|LiftMovement` :!via `Reverse` :!label _label)
        (:`Update`
          (`SceneComponent.K2_SetRelativeLocation` (`self.Base/LiftBody`) (`KismetMathLibrary.VLerp` (0.0 0.0 0.0) (0.0 0.0 4290.0) _alpha) false false))
        (:`Finished`
          ;;[0.08228 0.09759 0.15 0.502] Swap Lights back to red and set boolean on completed
          (for _ (`self.MeshesToUpdate`)
            (`PrimitiveComponent.SetMaterial` (`self.MeshesToUpdate`) 0 "/Game/Materials/MI_RedGlow.MI_RedGlow")
            (set `self.OnTopFloor?` true)))))
    (else
      (for _ (`self.MeshesToUpdate`)
        (`PrimitiveComponent.SetMaterial` (`self.MeshesToUpdate`) 0 "/Game/Materials/M_GlowingMaterial.M_GlowingMaterial")
        (goto _label)))))

(event `/Game/Blueprints/BPI_Interactable.OnInteract`
  (`self.MoveLift`))

(event `self.SwitchTrigger.OnComponentBeginOverlap`
  (params (OverlappedComponent :type "PrimitiveComponent Object Reference") (OtherActor :type "Actor Object Reference") (OtherComp :type "PrimitiveComponent Object Reference") (OtherBodyIndex :type Integer) (bFromSweep :type Boolean) (SweepResult :type "HitResult Structure (by ref)"))
  ; Overlap Logic, For Button, Show widget
  (cast `Character` OtherActor)
  (`self.EnableInput` (`GameplayStatics.GetPlayerController` 0))
  (`SceneComponent.SetVisibility` (`self.InteractWidget`) true false))

(event `self.ReceiveBeginPlay`
  ;[0.15 0.04219 0.1175 0.5] Fill Array Of switches that need to change colour
  (`|ExecutionSequence`
    (:`then_0`
      (set `self.MeshesToUpdate` (`self.GetComponentsByTag` "/Script/Engine.StaticMeshComponent" "LiftSwitch")))))

(event `self.SwitchTrigger.OnComponentEndOverlap`
  (params (OverlappedComponent :type "PrimitiveComponent Object Reference") (OtherActor :type "Actor Object Reference") (OtherComp :type "PrimitiveComponent Object Reference") (OtherBodyIndex :type Integer))
  ; Overlap Logic, For Button, Show widget
  (cast `Character` OtherActor)
  (`self.DisableInput` (`GameplayStatics.GetPlayerController` 0))
  (`SceneComponent.SetVisibility` (`self.InteractWidget`) false false))

(fn `UserConstructionScript`)