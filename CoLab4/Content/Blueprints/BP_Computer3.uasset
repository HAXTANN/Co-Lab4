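; Interactable downstairs computer that, one second after E is pressed, spends player attention, shuts down the downstairs machinery and signals completion.
; A trigger overlap toggles input and the prompt widget for characters.
; BeginPlay caches rotating-movement and light components from tagged actors.
; Activation deactivates the cached rotators, clears the lights' function materials to stop flicker and recolours them (blue, though comments say green).
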(event `Key|E`
  (params (Key :type "Key Structure"))
  ;[0.01687 0.15 0.02466 0.5] On Interact with Computer3
  (:`Pressed`
    (`KismetSystemLibrary.Delay` 1.0)
    (`self.SpendAttention`)
    (`self.Stop Rotating`)
    (`self.ChangeLights`)
    (set `self.ComputerActivated?` true)
    (`self.OnDownstairsComplete`)))

(event `StopRotatingActors`
  ;[0.15 0.016 0.09306 0.502] Rotating Actors
  ;;[0.15 0.016 0.09306 0.502] CustomEvent, create array get rotator and deactivate it
)

(event `self.Trigger.OnComponentBeginOverlap`
  (params (OverlappedComponent :type "PrimitiveComponent Object Reference") (OtherActor :type "Actor Object Reference") (OtherComp :type "PrimitiveComponent Object Reference") (OtherBodyIndex :type Integer) (bFromSweep :type Boolean) (SweepResult :type "HitResult Structure (by ref)"))
  ;[0.15 0.1353 0.03015 0.5] Interaction & Widget On/Off
  (cast `Character` OtherActor)
  (`self.EnableInput` (`GameplayStatics.GetPlayerController` 0))
  (`SceneComponent.SetVisibility` (`self.Widget`) true false))

(event `self.ReceiveBeginPlay`
  ;[0.15 0.016 0.09306 0.502] Rotating Actors
  ;;[0.15 0.016 0.09306 0.502] Stop Rotating Using an Array that you create and Store
  ;;;[0.15 0.016 0.09306 0.502] Premake Rotating Actor Array and Store it for Reference later
  (`|ExecutionSequence`
    (:`then_0`
      (`KismetArrayLibrary.Array_Clear` (`self.RotatingObjectsGroup`))
      (bind _outactors (`GameplayStatics.GetAllActorsWithTag` "RotatingActorsDownstairs"))
      (for _array_element _outactors
        (`KismetArrayLibrary.Array_Add` (`self.RotatingObjectsGroup`) (`self.GetComponentByClass` _array_element "/Script/Engine.RotatingMovementComponent"))))
    (:`then_1`
      ;[0.15 0.1274 0.05613 0.502] Lights
      ;;[0.15 0.1274 0.05613 0.502] Create and Store Array of lights that need to change
      (`KismetArrayLibrary.Array_Clear` (`self.RedToGreenLights`))
      (bind _outactors_2 (`GameplayStatics.GetAllActorsWithTag` "DownStairsRedLights"))
      (for _array_element_2 _outactors_2
        (`KismetArrayLibrary.Array_Add` (`self.RedToGreenLights`) (`self.GetComponentByClass` _array_element_2 "/Script/Engine.LocalLightComponent"))))))

(event `self.Trigger.OnComponentEndOverlap`
  (params (OverlappedComponent :type "PrimitiveComponent Object Reference") (OtherActor :type "Actor Object Reference") (OtherComp :type "PrimitiveComponent Object Reference") (OtherBodyIndex :type Integer))
  ;[0.15 0.1353 0.03015 0.5] Interaction & Widget On/Off
  (cast `Character` OtherActor)
  (`self.DisableInput` (`GameplayStatics.GetPlayerController` 0))
  (`SceneComponent.SetVisibility` (`self.Widget`) false false))

(event `Stop Rotating`
  ;[0.15 0.016 0.09306 0.502] Rotating Actors
  ;;[0.15 0.016 0.09306 0.502] Stop Rotating Using an Array that you create and Store
  ;;;[0.15 0.016 0.09306 0.502] StopRotating with Array Method
  (for _array_element (`self.RotatingObjectsGroup`)
    (`ActorComponent.Deactivate` _array_element)))

(event `SpendAttention`
  ;[0.15 0.04388 0.1128 0.5] Spend Attention CustomEvent
  (bind _asbp_first_person_character (cast `/Game/FirstPerson/Blueprints/BP_FirstPersonCharacter` (`GameplayStatics.GetPlayerCharacter` 0)))
  (`/Game/FirstPerson/Blueprints/BP_FirstPersonCharacter.ChangeAttention` _asbp_first_person_character -100.0))

(event `ChangeLights`
  ;[0.15 0.1274 0.05613 0.502] Lights
  ;;[0.15 0.1274 0.05613 0.502] Stop Lights Flickering and change their colour to Green
  (for _array_element (`self.RedToGreenLights`)
    (`LightComponent.SetLightFunctionMaterial` _array_element null)
    (`LightComponent.SetLightColor` _array_element (struct :`R` 0.111932 :`G` 0.351533 :`B` 1.0 :`A` 1.0) true)))

(fn `UserConstructionScript`)