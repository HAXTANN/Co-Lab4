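; BP_WaterRoomSwitch is an interactable switch that tells the water room computer to switch to the water wall.
; A trigger overlap by a Character enables input from player controller 0 and makes the trigger component visible.
; Ending the overlap disables that input and turns off only the interaction widget's ray tracing visibility.
; OnInteract calls SwitchToWaterWall on the referenced WaterRoomComputer.
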(event `/Game/Blueprints/BPI_Interactable.OnInteract`
  (`/Game/Blueprints/BP_WaterRoomComputer.SwitchToWaterWall` (`self.WaterRoomComputer`)))

(event `Key|One`
  (params (Key :type "Key Structure")))

(event `self.Trigger.OnComponentBeginOverlap`
  (params (OverlappedComponent :type "PrimitiveComponent Object Reference") (OtherActor :type "Actor Object Reference") (OtherComp :type "PrimitiveComponent Object Reference") (OtherBodyIndex :type Integer) (bFromSweep :type Boolean) (SweepResult :type "HitResult Structure (by ref)"))
  ;[0.15 0.04118 0.1182 0.5] Interaction Logic
  (cast `Character` OtherActor)
  (`self.EnableInput` (`GameplayStatics.GetPlayerController` 0))
  (`SceneComponent.SetVisibility` (`self.Trigger`) true false))

(event `self.Trigger.OnComponentEndOverlap`
  (params (OverlappedComponent :type "PrimitiveComponent Object Reference") (OtherActor :type "Actor Object Reference") (OtherComp :type "PrimitiveComponent Object Reference") (OtherBodyIndex :type Integer))
  ;[0.15 0.04118 0.1182 0.5] Interaction Logic
  (cast `Character` OtherActor)
  (`self.DisableInput` (`GameplayStatics.GetPlayerController` 0))
  (`PrimitiveComponent.SetVisibleInRayTracing` (`self.Interaction Widget`) false))

(fn `UserConstructionScript`)