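; BP_SplineCable is an actor that builds a chain of cable components along an editable spline.
; Its construction script makes each spline point linear and adds a cable from that point to the next.
; Each cable takes its width from CableThickness and its length from ExtraLength plus the current point's spline distance minus the next's, so the segment term is negative.
; The event graph holds no active logic.
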(fn `UserConstructionScript`
  (bind _cablespline (`self.CableSpline`))
  (bind _returnvalue (`SplineComponent.GetNumberOfSplinePoints` _cablespline))
  (for _index (range (+ _returnvalue 1))
    (`SplineComponent.SetSplinePointType` _cablespline _index "Linear" true)
    (bind _returnvalue_2 (+ _index 1))
    (if (< _returnvalue_2 _returnvalue)
      (bind (_returnvalue_inputkey _returnvalue_position) (break `SplinePoint` (`SplineComponent.GetSplinePointAt` _cablespline _index "Local")))
      (bind _returnvalue_3 (`AddComponent|NODE_AddCableComponent-0` :`RelativeTransform` (`KismetMathLibrary.Conv_VectorToTransform` _returnvalue_position)))
      (bind (_returnvalue_inputkey_2 _returnvalue_position_2) (break `SplinePoint` (`SplineComponent.GetSplinePointAt` _cablespline _returnvalue_2 "Local")))
      (set `CableComponent.EndLocation` _returnvalue_position_2 _returnvalue_3)
      (set `CableComponent.CableLength` (+ (- (`SplineComponent.GetDistanceAlongSplineAtSplinePoint` _cablespline _index) (`SplineComponent.GetDistanceAlongSplineAtSplinePoint` _cablespline _returnvalue_2)) (`self.ExtraLength`)) _returnvalue_3)
      (set `CableComponent.CableWidth` (`self.CableThickness`) _returnvalue_3))))