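; BP_LiftSwitch is an interactable switch that moves a referenced lift.
; A trigger volume detects overlapping Characters, enabling player input on the switch and showing an interaction widget, then reversing both when the overlap ends.
; While input is enabled, the OnInteract event calls MoveLift on the lift reference.
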(event `/Game/Blueprints/BPI_Interactable.OnInteract`
  (`/Game/Blueprints/BP_Lift.MoveLift` (`self.LiftReference`)))

(event `self.Trigger.OnComponentBeginOverlap`
  (params (OverlappedComponent :type "PrimitiveComponent Object Reference") (OtherActor :type "Actor Object Reference") (OtherComp :type "PrimitiveComponent Object Reference") (OtherBodyIndex :type Integer) (bFromSweep :type Boolean) (SweepResult :type "HitResult Structure (by ref)"))
  (cast `Character` OtherActor)
  (`self.EnableInput` (`GameplayStatics.GetPlayerController` 0))
  (`SceneComponent.SetVisibility` (`self.InteractionWidget`) true false))

(event `self.Trigger.OnComponentEndOverlap`
  (params (OverlappedComponent :type "PrimitiveComponent Object Reference") (OtherActor :type "Actor Object Reference") (OtherComp :type "PrimitiveComponent Object Reference") (OtherBodyIndex :type Integer))
  (cast `Character` OtherActor)
  (`self.DisableInput` (`GameplayStatics.GetPlayerController` 0))
  (`SceneComponent.SetVisibility` (`self.InteractionWidget`) false false))

(fn `UserConstructionScript`)