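; Base interactable actor that registers itself with the first-person character and shows an interaction prompt when in range.
; Sphere trigger overlap sets the character's CurrentInteractable to this actor, and end overlap clears it only if it still points here.
; ShowInteract and HideInteract toggle the InteractionWidget, gated on the overlapping character, rather than this actor, implementing BPI_Interactable.
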(event `/Game/Blueprints/BPI_Interactable.ShowInteract`
  (`SceneComponent.SetVisibility` (`self.InteractionWidget`) true false))

(event `/Game/Blueprints/BPI_Interactable.HideInteract`
  (`SceneComponent.SetVisibility` (`self.InteractionWidget`) false false))

(event `self.SphereTrigger.OnComponentBeginOverlap`
  (params (OverlappedComponent :type "PrimitiveComponent Object Reference") (OtherActor :type "Actor Object Reference") (OtherComp :type "PrimitiveComponent Object Reference") (OtherBodyIndex :type Integer) (bFromSweep :type Boolean) (SweepResult :type "HitResult Structure (by ref)"))
  (bind _asbp_first_person_character (cast `/Game/FirstPerson/Blueprints/BP_FirstPersonCharacter` OtherActor))
  (set `/Game/FirstPerson/Blueprints/BP_FirstPersonCharacter.CurrentInteractable` self _asbp_first_person_character)
  (if (`KismetSystemLibrary.DoesImplementInterface` OtherActor "/Game/Blueprints/BPI_Interactable.BPI_Interactable_C")
    (`/Game/Blueprints/BPI_Interactable.ShowInteract`)))

(event `self.SphereTrigger.OnComponentEndOverlap`
  (params (OverlappedComponent :type "PrimitiveComponent Object Reference") (OtherActor :type "Actor Object Reference") (OtherComp :type "PrimitiveComponent Object Reference") (OtherBodyIndex :type Integer))
  (bind _asbp_first_person_character (cast `/Game/FirstPerson/Blueprints/BP_FirstPersonCharacter` OtherActor))
  (if (== (`/Game/FirstPerson/Blueprints/BP_FirstPersonCharacter.CurrentInteractable` _asbp_first_person_character) self)
    (set `/Game/FirstPerson/Blueprints/BP_FirstPersonCharacter.CurrentInteractable` null _asbp_first_person_character)
    (if (`KismetSystemLibrary.DoesImplementInterface` OtherActor "/Game/Blueprints/BPI_Interactable.BPI_Interactable_C")
      (`/Game/Blueprints/BPI_Interactable.HideInteract`))))

(fn `UserConstructionScript`)