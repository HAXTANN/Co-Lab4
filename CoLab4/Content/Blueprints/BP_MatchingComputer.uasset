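; Matching computer that tracks whether a room's spot-the-difference items have all been fixed.
; UpdateRoomProgress counts entries in ItemsToFix whose BPC_DifferenceItem is correct, prints the tally, and on a full match calls the room-solved dispatcher and OnRoomComplete.
; OnRoomComplete is empty here, and CheckRoomStatus only prints "Room Matched" for each correct item rather than testing the whole room.
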(event `OnRoomComplete`)

(fn `CheckRoomStatus`
  (for _array_element (`self.ItemsToFix`)
    (if (`/Game/Blueprints/BPC_DifferenceItem.IsCorrect` (`self.GetComponentByClass` _array_element "/Game/Blueprints/BPC_DifferenceItem.BPC_DifferenceItem_C"))
      (`KismetSystemLibrary.PrintString` "Room Matched"))))

(fn `UpdateRoomProgress`
  (locals (Local_CorrectCount :type Integer))
  (set `local.Local_CorrectCount` 0)
  (for _array_element (`self.ItemsToFix`)
    (if (`/Game/Blueprints/BPC_DifferenceItem.IsCorrect` (`self.GetComponentByClass` _array_element "/Game/Blueprints/BPC_DifferenceItem.BPC_DifferenceItem_C"))
      (`/Engine/EditorBlueprintResources/StandardMacros.IncrementInt` (`local.Local_CorrectCount`))
      (else
        (`KismetSystemLibrary.PrintString` "Stilll More to do"))))
  (`KismetSystemLibrary.PrintString` (`KismetStringLibrary.Concat_StrStr` "Items Correct: " (`KismetStringLibrary.Conv_IntToString` (`local.Local_CorrectCount`)) " / " (`KismetStringLibrary.Conv_IntToString` (`KismetArrayLibrary.Array_Length` (`self.ItemsToFix`)))))
  (if (== (`KismetArrayLibrary.Array_Length` (`self.ItemsToFix`)) (`local.Local_CorrectCount`))
    (`self.RoomSolvedDispatcher`)
    (`self.OnRoomComplete`)))

(fn `UserConstructionScript`)