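; BP_WaterRoomComputer is a computer actor that switches the walls of a water room between solid glass and passable rippling water.
; On BeginPlay it gathers actors tagged WaterRoom and sets their static meshes to glass.
; Two custom events swap the material and collision on every wall, guarded by the WaterWallOn bool.
; The trigger overlap is an empty placeholder, and nothing in this graph calls the switch events.
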(event `self.ReceiveBeginPlay`
  ;[0.15 0.004391 0.004391 0.502] Get the list of walls and turn mesh to glass on start
  (`|ExecutionSequence`
    (:`then_0`
      (bind _outactors (`GameplayStatics.GetAllActorsWithTag` "WaterRoom"))
      (bind _output_get (set `self.WaterWalls` _outactors))
      (for _array_element _output_get
        (`PrimitiveComponent.SetMaterial` (`self.GetComponentByClass` _array_element "/Script/Engine.StaticMeshComponent") 0 "/Game/Fab/Light_bulb_High_Poly/light_bulb_high_poly/Materials/glass.glass")))))

(event `SwitchToWaterWall`
  ;[0.15 0.004391 0.004391 0.502] Turn on Water Walls custom Event and set bool
  (if (not (`self.WaterWallOn?`))
    (for _array_element (`self.WaterWalls`)
      (bind _returnvalue (`self.GetComponentByClass` _array_element "/Script/Engine.StaticMeshComponent"))
      (`PrimitiveComponent.SetMaterial` _returnvalue 0 "/Game/Materials/M_Rippls_Inst.M_Rippls_Inst")
      (`PrimitiveComponent.SetCollisionEnabled` _returnvalue "NoCollision")
      (set `self.WaterWallOn?` true))))

(event `SwitchToCustomWalls`
  ;[0.15 0.004391 0.004391 0.502] Turn off water walls and set custom event and set bool
  (if (`self.WaterWallOn?`)
    (for _array_element (`self.WaterWalls`)
      (bind _returnvalue (`self.GetComponentByClass` _array_element "/Script/Engine.StaticMeshComponent"))
      (`PrimitiveComponent.SetMaterial` _returnvalue 0 "/Game/Fab/Light_bulb_High_Poly/light_bulb_high_poly/Materials/glass.glass")
      (`PrimitiveComponent.SetCollisionEnabled` _returnvalue "QueryAndPhysics")
      (set `self.WaterWallOn?` false))))

(event `self.Trigger.OnComponentBeginOverlap`
  (params (OverlappedComponent :type "PrimitiveComponent Object Reference") (OtherActor :type "Actor Object Reference") (OtherComp :type "PrimitiveComponent Object Reference") (OtherBodyIndex :type Integer) (bFromSweep :type Boolean) (SweepResult :type "HitResult Structure (by ref)"))
  ; Overlap interact logic wont be final
)

(fn `UserConstructionScript`)